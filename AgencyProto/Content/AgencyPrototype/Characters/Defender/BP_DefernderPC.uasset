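; BP_DefernderPC is the Defender's player controller, switching possession between the character, a deployable drone and map cameras.
; An Occupied flag gates spawning a drone or entering the first BP_MapManager camera, and exiting re-possesses the saved pawn.
; BeginPlay initializes survivor vision through BPCSVRipApart and a material parameter collection, and creates the FPS HUD, exposed through text and progress-bar functions.
; Interact triggers the first BP_HackableConsole found, without a proximity check.
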(event EventBeginPlay
  (bind _self self)
  (Utilities|FlowControl|Sequence
    (:then_0
      ;[1 1 1] Survivor Vision Init
      (Class|BPIntSurvivorVisionCharacter|SetController(Message) (Pawn|GetControlledPawn) _self)
      (Default|Initialize (Variables|Default|GetBPC_SVRipApart) _self))
    (:then_1
      ;[1 1 1] Save Character Pawn Instance
      (Variables|Components|SetCharacter%20Pawn (Pawn|GetControlledPawn)))
    (:then_2
      (Rendering|Material|SetScalarParameterValue "/Game/SurvivorVision/Materials/SurvivorVision/Functions/MPC_SurvivorVisionParameters.MPC_SurvivorVisionParameters" "Intensity" 1.0 :!class /Script/Engine.KismetMaterialLibrary))
    (:then_3
      ;[1 1 1] Get Map Cameras
      (bind _outactors (Actor|GetAllActorsOfClass "/Game/AgencyPrototype/Blueprints/Managers/BP_MapManager.BP_MapManager_C"))
      (Variables|Camera|SetCameras (Variables|/Game/AgencyPrototype/Blueprints/Managers/BPC_MapAssets.BPC_MapAssets_C|GetCameras (Variables|/Game/AgencyPrototype/Blueprints/Managers/BP_MapManager.BP_MapManager_C|GetBPC_MapAssets (Utilities|Array|Get(acopy) _outactors)))))
    (:then_4
      (bind _returnvalue (UserInterface|CreateWidget "/Game/AgencyPrototype/Widgets/WBP_FPSHUD.WBP_FPSHUD_C"))
      (bind _output_get (Variables|Default|SetWidgetHUD _returnvalue))
      (UserInterface|Viewport|AddtoViewport _output_get 0))))

(event EventTick
  (params (DeltaSeconds :type Float%20%28single-precision%29)))

(event Input|ActionEvents|InputActionDeployDrone
  (params (Key :type Key%20Structure :default "None"))
  (bind _returnvalue (Pawn|GetControlledPawn))
  ;[1 1 1] Drone
  (:Pressed
    (if (not (Variables|Default|GetOccupied))
      ;;[1 1 1] Deploy Drone Character and set that as controlled drone
      (bind _returnvalue_2 (Game|SpawnActorfromClass "/Game/AgencyPrototype/Characters/Drone/BP_DroneCharacter.BP_DroneCharacter_C" (Math|Conversions|ToTransform(Vector) (Math|Transform|TransformLocation (Transformation|GetActorTransform _returnvalue) (* (Transformation|GetActorForwardVector _returnvalue) 5.0))) "AdjustIfPossibleButAlwaysSpawn" 0 0))
      (bind _output_get (Variables|Drone|SetCreated%20Drone _returnvalue_2))
      (Pawn|Possess _output_get)
      (Variables|Default|SetOccupied true))))

(event Input|ActionEvents|InputActionEnterCamera
  (params (Key :type Key%20Structure :default "None"))
  ;[1 1 1] Enter Cameras
  (:Pressed
    (if (not (Variables|Default|GetOccupied))
      (bind _aspawn (Utilities|Casting|CastToPawn (Utilities|Array|Get(acopy) (Utilities|Struct|BreakArrayOfActor (Variables|Camera|GetCameras)))))
      (bind _asbp_camera_base (Utilities|Casting|CastToBP_CameraBase _aspawn))
      (Default|BeginView _asbp_camera_base)
      (Pawn|Possess _asbp_camera_base)
      (Variables|Default|SetOccupied true))))

(event Input|ActionEvents|InputActionExitState
  (params (Key :type Key%20Structure :default "None"))
  ;[1 1 1] Leave Camera or Drone back to main body
  (:Pressed
    (if (Variables|Default|GetOccupied)
      (Pawn|Possess (Variables|Components|GetCharacter%20Pawn))
      (Variables|Default|SetOccupied false))))

(event Input|ActionEvents|InputActionInteract
  (params (Key :type Key%20Structure :default "None"))
  (:Pressed
    (bind _outactors (Actor|GetAllActorsOfClass "/Game/AgencyPrototype/Blueprints/BP_HackableConsole.BP_HackableConsole_C"))
    (bind _asbp_hackable_console (Utilities|Casting|CastToBP_HackableConsole (Utilities|Array|Get(acopy) _outactors)))
    (Default|InteractCalled _asbp_hackable_console)))

(fn ConstructionScript)

(fn DisplayTexttoHUD
  (params (TextToDisplay :type String))
  (Default|DisplayText (Variables|Default|GetWidgetHUD) TextToDisplay)
  (return))

(fn UpdateProcessBar
  (params (ProgramVisible :type ESlateVisibility%20Enum :default "Visible") (Percentage :type Float%20%28single-precision%29))
  (Default|UpdateProgress (Variables|Default|GetWidgetHUD) ProgramVisible Percentage)
  (return))