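; Player controller for attacker characters, layering attacker-specific setup on shared base controller logic.
; On BeginPlay it sends itself to the controlled pawn, initializes the BPCSVRipApart component for Survivor Vision, and caches the pawn both generically and as BP_BaseAttacker.
; BaseBeginPlay then runs only if that cast succeeds or as the next sequence step, and Interact input forwards to BaseInteract.
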(event EventBeginPlay
  (bind _returnvalue (Pawn|GetControlledPawn))
  (bind _self self)
  (Utilities|FlowControl|Sequence
    (:then_0
      ;[1 1 1] Survivor Vision Init
      (Class|BPIntSurvivorVisionCharacter|SetController(Message) _returnvalue _self)
      (Default|Initialize (Variables|Default|GetBPC_SVRipApart) _self))
    (:then_1
      ;[1 1 1] Save Character Pawn Instance
      (bind _output_get (Variables|Default|SetCharacter%20Pawn _returnvalue))
      ;[1 1 1] Save Attacker Class reference
      (bind _asbp_base_attacker (Utilities|Casting|CastToBP_BaseAttacker _output_get))
      (Variables|Default|SetPawnAsBaseAttack _asbp_base_attacker))
    (:then_2
      (CallFunction|BaseBeginPlay))))

(event EventTick
  (params (DeltaSeconds :type Float%20%28single-precision%29)))

(event Input|ActionEvents|InputActionInteract
  (params (Key :type Key%20Structure :default "None"))
  ;[1 1 1] Call Base Interact
  (:Pressed
    (CallFunction|BaseInteract)))

(fn ConstructionScript)