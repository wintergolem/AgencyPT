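; Base controller Blueprint that creates the FPS HUD widget on BeginPlay and exposes functions for other objects to drive it.
; Callers can show or clear prompt text, update a progress bar, and set the location label, which swaps between two supplied names.
; Text that expects a response stores its instigator and enables interaction, so Base_Interact calls InteractCalled on that instigator until the matching text is removed.
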(event Custom|Base_Interact
  (if (Variables|Default|GetInteractEnable)
    (Default|InteractCalled (Variables|Default|GetInteractInstigator))))

(event EventBeginPlay
  (CallFunction|BuildWidget))

(event EventTick
  (params (DeltaSeconds :type Float%20%28single-precision%29)))

(fn ConstructionScript)

(fn DisplayTexttoHUD
  (params (TextToDisplay :type String) (Instigator :type Interact%20Interface%20Interface) (ExpectResponse :type Boolean))
  (Default|DisplayText (Variables|Default|GetWidgetUI) TextToDisplay)
  (bind _output_get (Variables|Default|SetInteractEnable ExpectResponse))
  (if _output_get
    (Variables|Default|SetInteractInstigator Instigator))
  (return))

(fn RemoveTextfromHUD
  (params (TextToRemove :type String))
  (bind _widgetui (Variables|Default|GetWidgetUI))
  (if (Utilities|Enum|Equal(Enum) TextToRemove (Variables|/Game/AgencyPrototype/Widgets/WBP_FPSHUD.WBP_FPSHUD_C|GetTextDisplayed _widgetui))
    (Default|DisplayText _widgetui)
    (Variables|Default|SetInteractEnable false)
    (return)))

(fn UpdateProcessBar
  (params (Visiblity :type ESlateVisibility%20Enum :default "Visible") (New%20Percentage :type Float%20%28single-precision%29))
  (Default|UpdateProgress (Variables|Default|GetWidgetUI) Visiblity New%20Percentage)
  (return))

(fn BuildWidget
  (Development|PrintString "BaseConstruct")
  (bind _returnvalue (UserInterface|CreateWidget "/Game/AgencyPrototype/Widgets/WBP_FPSHUD.WBP_FPSHUD_C"))
  (bind _output_get (Variables|Default|SetWidgetUI _returnvalue))
  (UserInterface|Viewport|AddtoViewport _output_get 0)
  (return))

(fn SetLocationName
  (params (LocationOneName :type String) (LocationTwoName :type String))
  (if (Utilities|Enum|Equal(Enum) LocationOneName (Variables|Default|GetSubLocationName))
    (bind _output_get (Variables|Default|SetSubLocationName LocationTwoName))
    (Variables|/Game/AgencyPrototype/Widgets/WBP_FPSHUD.WBP_FPSHUD_C|SetLocationDisplayed (Variables|Default|GetWidgetUI) _output_get)
    (return)
    (else
      (bind _output_get_2 (Variables|Default|SetSubLocationName LocationOneName))
      (Variables|/Game/AgencyPrototype/Widgets/WBP_FPSHUD.WBP_FPSHUD_C|SetLocationDisplayed (Variables|Default|GetWidgetUI) _output_get_2)
      (return))))