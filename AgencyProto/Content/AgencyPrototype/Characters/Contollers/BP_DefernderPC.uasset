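; Player controller for the Defender character, handling gun fire and reload, interaction, drone deployment and security camera viewing.
; On BeginPlay it caches the defender pawn, initializes survivor vision and its material parameter, fetches map cameras from BP_MapManager and builds the widget.
; Deploying a drone or entering the first map camera possesses that pawn and sets an Occupied flag that blocks both actions and firing.
; Exiting repossesses the saved character pawn.
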(event Custom|Firing%20Bullet
  ;[1 1 1] Fire Gun
  (Default|FireGunAnim (Variables|Default|GetDefenderCharacter)))

(event EventBeginPlay
  (bind _self self)
  (Utilities|FlowControl|Sequence
    (:then_0
      ;[1 1 1] Survivor Vision Init
      (Class|BPIntSurvivorVisionCharacter|SetController(Message) (Pawn|GetControlledPawn) _self)
      (Default|Initialize (Variables|Default|GetBPC_SVRipApart) _self))
    (:then_1
      ;[1 1 1] Save Character Pawn Instance
      (bind _output_get (Variables|Components|SetCharacter%20Pawn (Pawn|GetControlledPawn)))
      ;[1 1 1] Save Defender Class reference
      (bind _asbp_base_defender (Utilities|Casting|CastToBP_BaseDefender _output_get))
      (Variables|Default|SetDefenderCharacter _asbp_base_defender))
    (:then_2
      (Rendering|Material|SetScalarParameterValue "/Game/SurvivorVision/Materials/SurvivorVision/Functions/MPC_SurvivorVisionParameters.MPC_SurvivorVisionParameters" "Intensity" 1.0 :!class /Script/Engine.KismetMaterialLibrary))
    (:then_3
      ;[1 1 1] Get Map Cameras
      (bind _outactors (Actor|GetAllActorsOfClass "/Game/AgencyPrototype/Blueprints/Managers/BP_MapManager.BP_MapManager_C"))
      (Variables|Camera|SetCameras (Variables|/Game/AgencyPrototype/Blueprints/Managers/BPC_MapAssets.BPC_MapAssets_C|GetCameras (Variables|/Game/AgencyPrototype/Blueprints/Managers/BP_MapManager.BP_MapManager_C|GetBPC_MapAssets (Utilities|Array|Get(acopy) _outactors)))))
    (:then_4
      (CallFunction|BuildWidget))))

(event EventTick
  (params (DeltaSeconds :type Float%20%28single-precision%29)))

(event Input|ActionEvents|InputActionDeployDrone
  (params (Key :type Key%20Structure :default "None"))
  (bind _returnvalue (Pawn|GetControlledPawn))
  ;[1 1 1] Drone
  (:Pressed
    (if (not (Variables|Default|GetOccupied))
      ;;[1 1 1] Deploy Drone Character and set that as controlled drone
      (bind _returnvalue_2 (Game|SpawnActorfromClass "/Game/AgencyPrototype/Characters/Drone/BP_DroneCharacter.BP_DroneCharacter_C" (Math|Conversions|ToTransform(Vector) (Math|Transform|TransformLocation (Transformation|GetActorTransform _returnvalue) (* (Transformation|GetActorForwardVector _returnvalue) 5.0))) "AdjustIfPossibleButAlwaysSpawn" 0 0))
      (bind _output_get (Variables|Drone|SetCreated%20Drone _returnvalue_2))
      (Pawn|Possess _output_get)
      (Variables|Default|SetOccupied true))))

(event Input|ActionEvents|InputActionEnterCamera
  (params (Key :type Key%20Structure :default "None"))
  ;[1 1 1] Enter Cameras
  (:Pressed
    (if (not (Variables|Default|GetOccupied))
      (bind _aspawn (Utilities|Casting|CastToPawn (Utilities|Array|Get(acopy) (Utilities|Struct|BreakArrayOfActor (Variables|Camera|GetCameras)))))
      (bind _asbp_camera_base (Utilities|Casting|CastToBP_CameraBase _aspawn))
      (Default|BeginView _asbp_camera_base)
      (Pawn|Possess _asbp_camera_base)
      (Variables|Default|SetOccupied true))))

(event Input|ActionEvents|InputActionExitState
  (params (Key :type Key%20Structure :default "None"))
  ;[1 1 1] Leave Camera or Drone back to main body
  (:Pressed
    (if (Variables|Default|GetOccupied)
      (Pawn|Possess (Variables|Components|GetCharacter%20Pawn))
      (Variables|Default|SetOccupied false))))

(event Input|ActionEvents|InputActionFire
  (params (Key :type Key%20Structure :default "None"))
  (bind _defendercharacter (Variables|Default|GetDefenderCharacter))
  (bind _addedgun (Variables|/Game/AgencyPrototype/Characters/Defender/BP_BaseDefender.BP_BaseDefender_C|GetAddedGun _defendercharacter))
  ;[1 1 1] Fire Gun
  (:Pressed
    (if (not (Variables|Default|GetOccupied))
      (Default|FireCalled _addedgun)))
  (:Released
    (Default|TriggerReleased _addedgun)))

(event Input|ActionEvents|InputActionInteract
  (params (Key :type Key%20Structure :default "None"))
  ;[1 1 1] Call Base Interact
  (:Pressed
    (CallFunction|BaseInteract)))

(event Input|ActionEvents|InputActionReload
  (params (Key :type Key%20Structure :default "None"))
  ;[1 1 1] Reload Gun
  (:Pressed
    (Default|CallReload (Variables|/Game/AgencyPrototype/Characters/Defender/BP_BaseDefender.BP_BaseDefender_C|GetAddedGun (Variables|Default|GetDefenderCharacter)))))

(fn ConstructionScript)