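; Prototype player controller that sets up Survivor Vision and lets the player switch between the main character and a drone.
; BeginPlay hands itself to the pawn and vision manager, caches the character pawn, and sets the Survivor Vision material parameter collection intensity.
; DeployDrone toggles possession: it spawns a new drone at the pawn's transform and possesses it, or repossesses the cached character without destroying the drone.
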(event EventBeginPlay
  (bind _self self)
  (Utilities|FlowControl|Sequence
    (:then_0
      ;[1 1 1] Survivor Vision Init
      (Class|BPIntSurvivorVisionCharacter|SetController(Message) (Pawn|GetControlledPawn) _self)
      (Default|Initialize (Variables|Default|GetSurvivorVisionManager) _self))
    (:then_1
      ;[1 1 1] Save Character Pawn Instance
      (Variables|Default|SetCharacter%20Pawn (Pawn|GetControlledPawn)))
    (:then_2
      (Rendering|Material|SetScalarParameterValue "/Game/SurvivorVision/Materials/SurvivorVision/Functions/MPC_SurvivorVisionParameters.MPC_SurvivorVisionParameters" "Intensity" 1.0 :!class /Script/Engine.KismetMaterialLibrary))))

(event EventTick
  (params (DeltaSeconds :type Float%20%28single-precision%29)))

(event Input|ActionEvents|InputActionDeployDrone
  (params (Key :type Key%20Structure :default "None"))
  ;[1 1 1] Drone
  (:Pressed
    (if (Variables|Default|GetInDrone)
      ;;[1 1 1] Set View back to Main Character
      (Pawn|Possess (Variables|Default|GetCharacter%20Pawn))
      (Variables|Default|SetInDrone false)
      (else
        ;;[1 1 1] Deploy Drone Character and set that as controlled drone
        (bind _returnvalue (Game|SpawnActorfromClass "/Game/AgencyPrototype/Characters/Drone/BP_DroneCharacter.BP_DroneCharacter_C" (Transformation|GetActorTransform (Pawn|GetControlledPawn)) "AdjustIfPossibleButAlwaysSpawn" 0 0))
        (bind _output_get (Variables|Default|SetCreated%20Drone _returnvalue))
        (Pawn|Possess _output_get)
        (Variables|Default|SetInDrone true)))))

(fn ConstructionScript)