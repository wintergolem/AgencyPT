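; BP_BaseCharacter is a base character Blueprint that provides ladder climbing and exposes remodel availability and prompt text through two destruction getters.
; EnterLadder stores the ladder points, teleports the character to an end, and switches to flying movement with gravity adjusted.
; MoveonLadder moves along the capsule's up vector until within a threshold distance of either end.
; ExitLadder then teleports to the bottom or top stand point and restores gravity and walking.
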(event EventBeginPlay)

(event Collision|EventActorBeginOverlap
  (params (OtherActor :type Actor%20Object%20Reference)))

(event EventTick
  (params (DeltaSeconds :type Float%20%28single-precision%29)))

(event EventEnterLadder
  (params (Bottom :type Vector :default "0, 0, 0") (Top :type Vector :default "0, 0, 0") (TopStandPoint :type Vector :default "0, 0, 0") (EnterTop :type Boolean))
  ;[1 1 1] Ladder Interface
  (bind _output_get (Variables|Ladder|SetLadderStartPoint Bottom))
  (Variables|Ladder|SetLadderEndPoint Top)
  (Variables|Ladder|SetLadderTopStandPoint TopStandPoint)
  (Variables|/Script/Engine.CharacterMovementComponent|SetGravityScale (Variables|Character|GetCharacterMovement) (Variables|Ladder|GetLadderGravityScale))
  (Variables|Ladder|SetOnLadder true)
  (if EnterTop
    (Transformation|SetActorLocation _output_get false true)
    (else
      (Transformation|SetActorLocation Top false true)))
  (Physics|SetEnableGravity (Variables|Collision|GetCapsuleComponent) false)
  (Pawn|Components|CharacterMovement|SetMovementMode (Variables|Character|GetCharacterMovement) "MOVE_Flying" 0))

(event EventMoveonLadder
  (params (Scale :type Float%20%28single-precision%29))
  ;[1 1 1] Ladder Interface
  (if (not (== Scale 0.0))
    (if (< Scale 0.0)
      ;;[1 1 1] Calculate exit bottom
      (if (<= (Math|Vector|VectorLength (- (Transformation|GetActorLocation) (Variables|Ladder|GetLadderStartPoint))) (Variables|Ladder|GetDistanceToGetUp))
        (CallFunction|ExitLadder false)
        (else
          ;;[1 1 1] Just Move along ladder
          (Pawn|Input|AddMovementInput (Math|Vector|GetUpVector (Variables|Collision|GetCapsuleComponent)) (* Scale (Variables|Ladder|GetLadderMoveSpeed)) true :!label _label)))
      (else
        ;;[1 1 1] Calculate exit top
        (if (<= (Math|Vector|VectorLength (- (Transformation|GetActorLocation) (Variables|Ladder|GetLadderEndPoint))) (Variables|Ladder|GetDistanceToGetUp))
          (CallFunction|ExitLadder true)
          (else
            (goto _label)))))))

(event EventExitLadder
  (params (ExitTop :type Boolean))
  ;[1 1 1] Ladder Interface
  ;;[1 1 1] Exit Ladder
  (if ExitTop
    (Transformation|SetActorLocation (Variables|Ladder|GetLadderTopStandPoint) false true)
    (else
      (Transformation|SetActorLocation (Variables|Ladder|GetLadderStartPoint) false true)))
  (Variables|Ladder|SetOnLadder false)
  (Variables|/Script/Engine.CharacterMovementComponent|SetGravityScale (Variables|Character|GetCharacterMovement) (Variables|Ladder|GetStartGravityScale))
  (Physics|SetEnableGravity (Variables|Collision|GetCapsuleComponent) true)
  (Pawn|Components|CharacterMovement|SetMovementMode (Variables|Character|GetCharacterMovement) "MOVE_Walking" 0))

(fn ConstructionScript)

(fn DestructionAvailable
  (return (Variables|Remodel|GetRemodelAvailable)))

(fn DestructionPromptText
  (return (Variables|Remodel|GetRemodelPrompt)))