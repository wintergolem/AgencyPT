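; BP_CameraBase is a camera Blueprint, apparently a base class, that applies a desaturation post-process look.
; On BeginPlay it creates a dynamic instance of MI_SV_Camera and registers it on its PostProcess component at full weight.
; BeginView sets that instance's desaturation amount and intensity parameters, then re-applies the blendable.
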(event EventBeginPlay
  (bind _returnvalue (Rendering|Material|CreateDynamicMaterialInstance "/Game/AgencyPrototype/Materials/MI_SV_Camera.MI_SV_Camera" "None" :!class /Script/Engine.KismetMaterialLibrary))
  (bind _output_get (Variables|Default|SetDynMat _returnvalue))
  (Rendering|AddorUpdateBlendable (Variables|Default|GetPostProcess) _output_get 1.0 :!class /Script/Engine.PostProcessComponent))

(fn ConstructionScript)

(fn BeginView
  (bind _dynmat (Variables|Default|GetDynMat))
  (Rendering|Material|SetScalarParameterValue _dynmat "Desaturation Amount" 1.0 :!class /Script/Engine.MaterialInstanceDynamic)
  (Rendering|Material|SetScalarParameterValue _dynmat "desaturation intensity" 0.6 :!class /Script/Engine.MaterialInstanceDynamic)
  (Rendering|AddorUpdateBlendable (Variables|Default|GetPostProcess) _dynmat 1.0 :!class /Script/Engine.PostProcessComponent)
  (return))