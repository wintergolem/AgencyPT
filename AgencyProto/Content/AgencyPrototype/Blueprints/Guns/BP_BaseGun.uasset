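; Base gun Blueprint that handles automatic fire and delayed reloading for the defender's weapons.
; On BeginPlay it derives the shot interval from BulletsPerSecond; FireCalled fires immediately, then repeats FireShots on a looping timer until TriggerReleased clears it.
; Each successful TriggerPull notifies DefenderPC through FiringBullet.
; CallReload schedules Reload by name after ReloadTimeInSeconds; neither Reload nor TriggerPull is defined in this graph.
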(event Custom|FireCalled
  (CallFunction|FireShots)
  (bind _returnvalue (Utilities|Time|SetTimerbyFunctionName 0 "FireShots" (Variables|Default|GetTImeBetweenBullets) true))
  (Variables|Default|SetFireTimer _returnvalue))

(event Custom|TriggerReleased
  (Utilities|Time|ClearandInvalidateTimerbyHandle (Variables|Default|GetFireTimer)))

(event Custom|CallReload
  (Utilities|Time|SetTimerbyFunctionName 0 "Reload" (Variables|Default|GetReloadTimeInSeconds)))

(event EventBeginPlay
  (Variables|Default|SetTImeBetweenBullets (/ 1.0 (Variables|Default|GetBulletsPerSecond))))

(event Collision|EventActorBeginOverlap
  (params (OtherActor :type Actor%20Object%20Reference)))

(event EventTick
  (params (DeltaSeconds :type Float%20%28single-precision%29)))

(fn ConstructionScript)

(fn FireShots
  (bind _returnvalue (Class|BaseGun|TriggerPull))
  (if _returnvalue
    (Default|FiringBullet (Variables|Default|GetDefenderPC))))