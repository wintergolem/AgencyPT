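; BP_HackableConsole is a console the player can start hacking by interacting inside a start trigger volume.
; The start volume shows the prompt and permits interaction, while a separate area volume handles hacking text and clears the active state on exit.
; Tick pushes hack progress to the player controller's HUD widget while the hack is started and active.
; Nothing in this graph advances the percentage, sets the hack active or completes it.
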(event OnComponentBeginOverlap(HackStartTriggerVolume)
  (params (OverlappedComponent :type Primitive%20Component%20Object%20Reference) (OtherActor :type Actor%20Object%20Reference) (OtherComp :type Primitive%20Component%20Object%20Reference) (OtherBodyIndex :type Integer) (bFromSweep :type Boolean) (SweepResult :type Hit%20Result%20Structure%20%28by%20ref%29))
  (Default|DisplayTexttoHUD (Variables|Default|GetPlayerController) (Variables|Default|GetInteractText) self true)
  (Variables|Default|SetPlayerCanStartHack true))

(event OnComponentEndOverlap(HackStartTriggerVolume)
  (params (OverlappedComponent :type Primitive%20Component%20Object%20Reference) (OtherActor :type Actor%20Object%20Reference) (OtherComp :type Primitive%20Component%20Object%20Reference) (OtherBodyIndex :type Integer))
  (Default|RemoveTextfromHUD (Variables|Default|GetPlayerController) (Variables|Default|GetInteractText))
  (Variables|Default|SetPlayerCanStartHack false))

(event OnComponentEndOverlap(HackAreaTriggerVolume)
  (params (OverlappedComponent :type Primitive%20Component%20Object%20Reference) (OtherActor :type Actor%20Object%20Reference) (OtherComp :type Primitive%20Component%20Object%20Reference) (OtherBodyIndex :type Integer))
  (bind _playercontroller (Variables|Default|GetPlayerController))
  (Default|UpdateProcessBar _playercontroller "Hidden" 0.0)
  (Default|RemoveTextfromHUD _playercontroller (Variables|Default|GetInteractintText))
  (Variables|Default|SetHackActive false))

(event OnComponentBeginOverlap(HackAreaTriggerVolume)
  (params (OverlappedComponent :type Primitive%20Component%20Object%20Reference) (OtherActor :type Actor%20Object%20Reference) (OtherComp :type Primitive%20Component%20Object%20Reference) (OtherBodyIndex :type Integer) (bFromSweep :type Boolean) (SweepResult :type Hit%20Result%20Structure%20%28by%20ref%29))
  (if (Variables|Default|GetHackStarted)
    (Default|DisplayTexttoHUD (Variables|Default|GetPlayerController) (Variables|Default|GetInteractintText) 0 false)))

(event EventBeginPlay
  (bind _asbp_base_cc (Utilities|Casting|CastToBP_BaseCC (Game|GetPlayerController 0)))
  (Variables|Default|SetPlayerController _asbp_base_cc))

(event EventInteractCalled
  (bind _playercontroller (Variables|Default|GetPlayerController))
  (if (Variables|Default|GetPlayerCanStartHack)
    (Variables|Default|SetHackStarted true)
    (Default|RemoveTextfromHUD _playercontroller (Variables|Default|GetInteractText))
    (Default|DisplayTexttoHUD _playercontroller "Hacking..." 0 false)))

(event EventTick
  (params (DeltaSeconds :type Float%20%28single-precision%29))
  (bind _playercontroller (Variables|Default|GetPlayerController))
  (if (and (Variables|Default|GetHackActive) (Variables|Default|GetHackStarted))
    (Default|UpdateProgress (Variables|/Game/AgencyPrototype/Characters/Contollers/BP_BaseCC.BP_BaseCC_C|GetWidgetUI _playercontroller) "Visible" (Variables|Default|GetHackTimePercentage))
    (else
      (Default|UpdateProgress (Variables|/Game/AgencyPrototype/Characters/Contollers/BP_BaseCC.BP_BaseCC_C|GetWidgetUI _playercontroller) "Hidden" 0.0))))

(fn ConstructionScript)